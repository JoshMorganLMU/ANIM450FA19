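; Interactable lamp actor that toggles its point light on and off, with the initial state set from IsOn in the construction script.
; On BeginPlay it caches BP_GameMode_Interact, which acts as the interaction hub.
; Overlapping InteractCollider binds InteractEvt to the game mode's dispatcher, notifies it and reveals the collider; ending overlap reverses this.
; Both InteractEvt and a separate Interact event call ToggleLamp, which also prints the new state.
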(event `self.ReceiveBeginPlay`
  (`KismetSystemLibrary.PrintString` (`KismetSystemLibrary.GetDisplayName` self))
  (bind _asbp_game_mode_interact (cast `/Game/_BP/Modes/BP_GameMode_Interact` (`GameplayStatics.GetGameMode`)))
  (set `self.GameMode_Interact` _asbp_game_mode_interact))

(event `InputAction|LampInteract`
  (params (Key :type "Key Structure")))

(event `self.InteractCollider.OnComponentBeginOverlap`
  (params (OverlappedComponent :type "PrimitiveComponent Object Reference") (OtherActor :type "Actor Object Reference") (OtherComp :type "PrimitiveComponent Object Reference") (OtherBodyIndex :type Integer) (bFromSweep :type Boolean) (SweepResult :type "HitResult Structure (by ref)"))
  ;[1 1 1] BoxCollider Overlap
  (add `/Game/_BP/Modes/BP_GameMode_Interact.InteractEvtDispatch` (`self.GameMode_Interact`) (delegate `InteractEvt`))
  (`/Game/_BP/Modes/BP_GameMode_Interact.InteractiveCollisionBeginEvt` (`self.GameMode_Interact`))
  (`SceneComponent.SetHiddenInGame` (`self.InteractCollider`) false false))

(event `self.InteractCollider.OnComponentEndOverlap`
  (params (OverlappedComponent :type "PrimitiveComponent Object Reference") (OtherActor :type "Actor Object Reference") (OtherComp :type "PrimitiveComponent Object Reference") (OtherBodyIndex :type Integer))
  ;[1 1 1] BoxCollider Overlap
  (remove `/Game/_BP/Modes/BP_GameMode_Interact.InteractEvtDispatch` (`self.GameMode_Interact`) (delegate `InteractEvt`))
  (`/Game/_BP/Modes/BP_GameMode_Interact.InteractiveCollisionEndEvt` (`self.GameMode_Interact`))
  (`SceneComponent.SetHiddenInGame` (`self.InteractCollider`) true false))

(event `InteractEvt`
  ;[1 1 1] InteractEvt
  (`self.ToggleLamp`))

(event `/Game/_BP/Interfaces/BP_Interact_Interface.Interact`
  (`self.ToggleLamp`))

(fn `ToggleLamp`
  (bind _output_get (set `self.IsOn` (not (`self.IsOn`))))
  (`SceneComponent.SetVisibility` (`self.PointLight`) _output_get false)
  (`KismetSystemLibrary.PrintString` (`KismetStringLibrary.Concat_StrStr` "Turn Lamp " (select `bool` (`self.IsOn`) :`false` "OFF" :`true` "ON"))))

(fn `UserConstructionScript`
  (`SceneComponent.SetVisibility` (`self.PointLight`) (`self.IsOn`) false))