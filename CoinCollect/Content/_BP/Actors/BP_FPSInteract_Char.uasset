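; First-person player character with axis-driven movement, mouse look and a health value that drains every frame.
; Its InteractCollider overlap checks the other actor's interface and component name to send either an interact message or random damage.
; Health starts at max on BeginPlay and drops on Tick without delta-time scaling, clamping or death handling.
; Overlaps also print debug strings.
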(event `self.ReceiveBeginPlay`
  (`self.EnableInput` (`GameplayStatics.GetPlayerController` 0))
  (set `self.HealthCurrent` (`self.HealthMax`)))

(event `InputAxis|MoveForward`
  (params (AxisValue :type "Float (single-precision)"))
  ;[1 1 1] Move Controls
  (`self.AddMovementInput` (`KismetMathLibrary.GetForwardVector` (`self.GetControlRotation`)) AxisValue))

(event `InputAxis|MoveRight`
  (params (AxisValue :type "Float (single-precision)"))
  ;[1 1 1] Move Controls
  (`self.AddMovementInput` (`KismetMathLibrary.GetRightVector` (`self.GetControlRotation`)) AxisValue))

(event `InputAxis|LookHoriz`
  (params (AxisValue :type "Float (single-precision)"))
  ;[1 1 1] Look with Mouse Controls
  (`self.AddControllerYawInput` AxisValue))

(event `InputAxis|LookVert`
  (params (AxisValue :type "Float (single-precision)"))
  ;[1 1 1] Look with Mouse Controls
  (`self.AddControllerPitchInput` AxisValue))

(event `self.InteractCollider.OnComponentBeginOverlap`
  (params (OverlappedComponent :type "PrimitiveComponent Object Reference") (OtherActor :type "Actor Object Reference") (OtherComp :type "PrimitiveComponent Object Reference") (OtherBodyIndex :type Integer) (bFromSweep :type Boolean) (SweepResult :type "HitResult Structure (by ref)"))
  (`|ExecutionSequence`
    (:`then_0`
      (`KismetSystemLibrary.PrintString` (`KismetSystemLibrary.GetObjectName` OtherComp)))
    (:`then_1`
      (if (`KismetSystemLibrary.DoesImplementInterface` OtherActor "/Game/_BP/Interfaces/BP_Interact_Interface.BP_Interact_Interface_C")
        (`|ExecutionSequence`
          (:`then_0`
            (`KismetSystemLibrary.PrintString` "Is INTERACTIVE"))
          (:`then_1`
            (if (`KismetStringLibrary.EqualEqual_StrStr` (`KismetSystemLibrary.GetObjectName` OtherComp) "InteractCollider")
              (message `/Game/_BP/Interfaces/BP_Interact_Interface.Interact` OtherActor))))))
    (:`then_2`
      (if (and (`KismetSystemLibrary.DoesImplementInterface` OtherActor "/Game/_BP/Interfaces/BP_Damageable_Interface.BP_Damageable_Interface_C") (`KismetStringLibrary.EqualEqual_StrStr` (`KismetSystemLibrary.GetObjectName` OtherComp) "DamageCollider"))
        (message `/Game/_BP/Interfaces/BP_Damageable_Interface.TakeDamage` OtherActor (`KismetMathLibrary.RandomIntegerInRange` 10 50))))))

(event `self.ReceiveTick`
  (params (DeltaSeconds :type "Float (single-precision)"))
  (set `self.HealthCurrent` (- (`self.HealthCurrent`) (`self.HealthDrain`))))

(fn `UserConstructionScript`)