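; Game mode for the Interact mode that manages the interaction popup UI and a play-time countdown.
; On BeginPlay it shows the mouse cursor, creates the main HUD and popup menu widgets, and starts a looping one-second timer.
; Collision begin and end events adjust an overlap counter, so the popup stays visible until no interactive collisions remain.
; The timer decrements remaining time and only prints it, plus "Game Over" at zero, without stopping.
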(event `self.ReceiveBeginPlay`
  (set `PlayerController.bShowMouseCursor` true (`GameplayStatics.GetPlayerController` 0))
  (bind _returnvalue (`|CreateWidget` "/Game/_BP/UI/BP_Interact_PopupMenu.BP_Interact_PopupMenu_C"))
  (set `self.InteractMainUI` _returnvalue)
  (bind _returnvalue_2 (`|CreateWidget` "/Game/_BP/UI/BP_Interact_MainHUD.BP_Interact_MainHUD_C"))
  (`UserWidget.AddToViewport` _returnvalue_2 0)
  (set `self.PlayTimeSecondsRemaining` (`self.PlayTimeSecondsMax`))
  (`KismetSystemLibrary.K2_SetTimer` null "DecrementPlayTime" 1.0 true))

(event `ShowInteractUIEvt`
  (if (not (`Widget.IsInViewport` (`self.InteractMainUI`)))
    (`UserWidget.AddToViewport` (`self.InteractMainUI`) 0)))

(event `HideInteractUIEvt`
  (if (and (`Widget.IsInViewport` (`self.InteractMainUI`)) (== (`self.InteractiveCollisionCount`) 0))
    (`Widget.RemoveFromParent` (`self.InteractMainUI`))))

(event `IncrementInteractiveCollisionCountEvt`
  (`/Engine/EditorBlueprintResources/StandardMacros.IncrementInt` (`self.InteractiveCollisionCount`)))

(event `DecrementInteractiveCollisionCountEvt`
  (`/Engine/EditorBlueprintResources/StandardMacros.DecrementInt` (`self.InteractiveCollisionCount`)))

(event `InteractiveCollisionBeginEvt`
  (`self.IncrementInteractiveCollisionCountEvt`)
  (`self.ShowInteractUIEvt`))

(event `InteractiveCollisionEndEvt`
  (`self.DecrementInteractiveCollisionCountEvt`)
  (`self.HideInteractUIEvt`))

(fn `DecrementPlayTime`
  (bind _playtimesecondsremaining (`self.PlayTimeSecondsRemaining`))
  (`/Engine/EditorBlueprintResources/StandardMacros.DecrementInt` _playtimesecondsremaining
    (:`  `
      (`KismetSystemLibrary.PrintString` (`KismetStringLibrary.Conv_IntToString` _playtimesecondsremaining))
      (if (<= _playtimesecondsremaining 0)
        (`KismetSystemLibrary.PrintString` "Game Over")))))

(fn `UserConstructionScript`)