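; Blueprint function library with two small general-purpose helpers.
; PadZerosIntAsStr converts an integer to a string and prepends zeros until it reaches a given digit count.
; RandomActorInArray returns a randomly chosen element from an actor array, with no check for an empty array.
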(fn `PadZerosIntAsStr`
  (params (IntToPad :type Integer) (NumDigits :type Integer))
  (returns (PaddedIntAsStr :type String))
  (locals (IntAsStr :type String))
  (bind _output_get (set `local.IntAsStr` (`KismetStringLibrary.Conv_IntToString` IntToPad)))
  (while (< (`KismetStringLibrary.Len` _output_get) NumDigits)
    (set `local.IntAsStr` (`KismetStringLibrary.Concat_StrStr` "0" (`local.IntAsStr`))))
  (return (`local.IntAsStr`)))

(fn `RandomActorInArray`
  (params (ActorArray :type "Array of Actor Object Reference"))
  (returns (NewParam :type "Actor Object Reference"))
  (return (`|GetArrayItem` ActorArray (`KismetMathLibrary.RandomInteger` (`KismetArrayLibrary.Array_Length` ActorArray)))))